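; Item_BP is a configurable physics item that BP_MotionController can pick up and drop.
; On BeginPlay it applies its mesh and main material, using the Russian Type string to choose the slot: the second for liquid or flask, the first otherwise.
; Spheres also show a particle system.
; Pickup disables physics and attaches the root to the given component, while Drop re-enables physics and detaches, both keeping world transform.
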(event EventBeginPlay
  (Variables|Default|Setname (Variables|Default|Getname))
  (bind _output_get (Variables|Default|Settype (Variables|Default|Gettype)))
  (Components|StaticMesh|SetStaticMesh (Variables|Debug|GetStaticMeshComponent) (Variables|Default|GetmyMesh))
  (if (Utilities|Enum|Equal(Enum) _output_get "Жидкость")
    (Rendering|Material|SetMaterial (Variables|Debug|GetStaticMeshComponent) 1 (Variables|Default|GetmaterialMain) :!label _label)
    (elif (Utilities|Enum|Equal(Enum) _output_get "Колба")
      (goto _label)
      (elif (Utilities|Enum|Equal(Enum) _output_get "Сфера")
        (Rendering|Material|SetMaterial (Variables|Debug|GetStaticMeshComponent) 0 (Variables|Default|GetmaterialMain))
        (Variables|Default|SetmyParticleSystem (Variables|Default|GetmyParticleSystem))
        (Rendering|SetVisibility (Variables|Default|GetmyParticleSystem) true false)
        (else
          (Rendering|Material|SetMaterial (Variables|Debug|GetStaticMeshComponent) 0 (Variables|Default|GetmaterialMain)))))))

(event EventPickup
  (params (MotionControllerReference :type BP%20Motion%20Controller%20Object%20Reference) (AttachTo :type Scene%20Component%20Object%20Reference))
  (Physics|SetSimulatePhysics (Variables|Debug|GetStaticMeshComponent) false)
  (Transformation|AttachComponentToComponent (VehicleSound|GetRootComponent) AttachTo "None" "KeepWorld" "KeepWorld" "KeepWorld" false))

(event EventDrop
  (Physics|SetSimulatePhysics (Variables|Debug|GetStaticMeshComponent) true)
  (Transformation|DetachFromActor "KeepWorld" "KeepWorld" "KeepWorld"))

(fn ConstructionScript)