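; Potion cauldron that mixes dropped Item_BP liquids, tracks the current potion, and turns it into spheres or filled flasks.
; Shaker overlap mixes liquids via an order-independent dictionary recipe lookup, recoloring water and bubbles through dynamic materials; failed mixes turn brown.
; A catalyst looks up a result item to spawn and empties the water.
; Grub overlap fills flasks from the same item dictionary, copying color and emptying the cauldron.
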(event OnComponentBeginOverlap(Grub)
  (params (OverlappedComponent :type Primitive%20Component%20Object%20Reference) (OtherActor :type Actor%20Object%20Reference) (OtherComp :type Primitive%20Component%20Object%20Reference) (OtherBodyIndex :type Integer) (bFromSweep :type Boolean) (SweepResult :type Hit%20Result%20Structure%20%28by%20ref%29))
  ;[1 1 1] Поверхность: если вода есть - значит её можно набрать =>
  (if (Variables|Default|GetisWater?)
    ;[1 1 1] Налить жидкость можно только в колбу, это круто!
    (bind _asitem_bp (Utilities|Casting|CastToItem_BP OtherActor))
    (if (Utilities|Enum|Equal(Enum) (Variables|/Game/Old/BP/Item_BP.Item_BP_C|Gettype _asitem_bp) "Колба")
      ;[1 1 1] Ищем, можно ли налить в колбу жидкость
      (bind (_result _find_) (Utilities|GetNewItem (Variables|/Game/Old/BP/Item_BP.Item_BP_C|Gettype _asitem_bp))
        (:Output
          (if _find_
            (bind _output_get (Variables|/Game/Old/BP/Item_BP.Item_BP_C|Setname _asitem_bp (.name (Utilities|Struct|BreakResult _result))))
            (bind _new_color (Utilities|WaterColor _output_get)
              (:Out
                ;[1 1 1] Если такая штука найдена, то подменяем параметры колбы на новые
                (Variables|/Game/Old/BP/Item_BP.Item_BP_C|Settype _asitem_bp (.type (Utilities|Struct|BreakResult _result)))
                (Rendering|Material|SetMaterial (Variables|/Script/Engine.StaticMeshActor|GetStaticMeshComponent _asitem_bp) 1 (.materialMain (Utilities|Struct|BreakResult _result)))
                (bind _returnvalue (Rendering|Material|CreateDynamicMaterialInstance (Variables|/Script/Engine.StaticMeshActor|GetStaticMeshComponent _asitem_bp) 2 "/Game/Assets/SceneMaterial/Material/MaterialBubl_PotterWater.MaterialBubl_PotterWater" "" :!class /Script/Engine.PrimitiveComponent))
                (Rendering|Material|SetVectorParameterValue _returnvalue "color" (Math|Conversions|ToLinearColor(Color) _new_color) :!class /Script/Engine.MaterialInstanceDynamic)
                (Variables|/Game/Old/BP/Item_BP.Item_BP_C|Setrgb _asitem_bp (Math|Conversions|ToColor(LinearColor) (Math|Conversions|ToLinearColor(Color) _new_color)))
                ;;[1 1 1] Убираем воду
                (Variables|Default|SetisWater? false)
                (Rendering|SetVisibility (Variables|Default|Getcotl_water) false true)
                (Development|PrintString _output_get)))
            (else
              ;[1 1 1] Чистим котел
              (Variables|Default|SetisWater? false)
              (Rendering|SetVisibility (Variables|Default|Getcotl_water) false false)
              (Variables|Default|SetCurrentPotion "")
              (Development|PrintString "6: Что то пошло не так"))))))))

(event OnComponentBeginOverlap(Shaker)
  (params (OverlappedComponent :type Primitive%20Component%20Object%20Reference) (OtherActor :type Actor%20Object%20Reference) (OtherComp :type Primitive%20Component%20Object%20Reference) (OtherBodyIndex :type Integer) (bFromSweep :type Boolean) (SweepResult :type Hit%20Result%20Structure%20%28by%20ref%29))
  ;[1 1 1] Дно чана: проверяем чем является кинутый предмет (жидкость или катализатор)
  (bind _asitem_bp (Utilities|Casting|CastToItem_BP OtherActor))
  (if (Utilities|Enum|Equal(Enum) (Variables|/Game/Old/BP/Item_BP.Item_BP_C|Gettype _asitem_bp) "Жидкость")
    ;[1 1 1] Жидкость: Если есть вода - значит пытаемся смешать зелья. Если воды нет - значит это первое зелье в рецепте.
    (if (Variables|Default|GetisWater?)
      (bind (_new_potion _find_) (Utilities|ShakePotions (Variables|/Game/Old/BP/Item_BP.Item_BP_C|Getname _asitem_bp))
        (:Out
          ;[1 1 1] Получем новую жидкость и смотрим на её цвет. В верхней ветке: если жидкость не надена, то вода становится грязной, а целевой результат провальным => спускаемся в нижний блок
          (if _find_
            (bind _output_get (Variables|Default|SetCurrentPotion _new_potion))
            (bind _new_color (Utilities|WaterColor _output_get)
              (:Out
                (Variables|Default|SetnewRGB _new_color)
                ;[1 1 1] Делаем видимой воду и пузырьки, если это первое зелье в рецепте. Устанавливаем им новый цвет.
                (bind _returnvalue (Rendering|Material|CreateDynamicMaterialInstance (Variables|Default|Getcotl_water) 0 "/Game/Assets/SceneMaterial/Material/MaterialBubl_PotterWater.MaterialBubl_PotterWater" "" :!class /Script/Engine.PrimitiveComponent :!label _label))
                (Rendering|Material|SetVectorParameterValue _returnvalue "color" (Math|Conversions|ToLinearColor(Color) (Variables|Default|GetnewRGB)) :!class /Script/Engine.MaterialInstanceDynamic)
                (bind _returnvalue_2 (Rendering|Material|CreateDynamicMaterialInstance (Variables|Default|GetParticlBubl) 0 "/Game/Old/Particle/Material/Shader/ShaderBubl_Inst.ShaderBubl_Inst" "" :!class /Script/Engine.PrimitiveComponent))
                (Rendering|Material|SetVectorParameterValue _returnvalue_2 "color" (Math|Conversions|ToLinearColor(Color) (Variables|Default|GetnewRGB)) :!class /Script/Engine.MaterialInstanceDynamic)
                (Actor|DestroyActor _asitem_bp)
                ;[1 1 1] Название нового зелья
                (Development|PrintString (Variables|Default|GetCurrentPotion))))
            (else
              ;[1 1 1] Если новая жидкость не получилась - значит красим воду в коричневый цвет
              (Variables|Default|SetCurrentPotion "")
              (bind _returnvalue_3 (Rendering|Material|CreateDynamicMaterialInstance (Variables|Default|Getcotl_water) 0 0 "" :!class /Script/Engine.PrimitiveComponent))
              (Rendering|Material|SetVectorParameterValue _returnvalue_3 "color" "(R=0.104616,G=0.034340,B=0.000000,A=1.000000)" :!class /Script/Engine.MaterialInstanceDynamic)
              (bind _returnvalue_4 (Rendering|Material|CreateDynamicMaterialInstance (Variables|Default|GetParticlBubl) 0 0 "" :!class /Script/Engine.PrimitiveComponent))
              (Rendering|Material|SetVectorParameterValue _returnvalue_4 "color" "(R=0.104616,G=0.034340,B=0.000000,A=1.000000)" :!class /Script/Engine.MaterialInstanceDynamic)
              (Actor|DestroyActor _asitem_bp)
              (Development|PrintString "4: Отлично, вы свариили како-то дерьмо!")))))
      (else
        (bind _output_get_2 (Variables|Default|SetCurrentPotion (Variables|/Game/Old/BP/Item_BP.Item_BP_C|Getname _asitem_bp)))
        (bind _new_color_2 (Utilities|WaterColor _output_get_2)
          (:Out
            (Variables|Default|SetnewRGB _new_color_2)
            (Variables|Default|SetisWater? true)
            (Rendering|SetVisibility (Variables|Default|Getcotl_water) true true)
            (goto _label)))))
    (elif (Utilities|Enum|Equal(Enum) (Variables|/Game/Old/BP/Item_BP.Item_BP_C|Gettype _asitem_bp) "Катализатор")
      ;[1 1 1] Если в котел попал катализатор и в котле есть жидкость - смотрим, получится ли из него что-то, если жидкости нет, то пусть валяется на дне
      (if (Variables|Default|GetisWater?)
        (bind (_result _find__2) (Utilities|GetNewItem "Катализатор")
          (:Output
            (if _find__2
              ;[1 1 1] Если был найден хотя бы один результат от смешивания катализатора с водой, то создаем сферу с партиклом внутри
              (bind _returnvalue_5 (Game|SpawnActorfromClass "/Game/Old/BP/Item_BP.Item_BP_C" (Math|Conversions|ToTransform(Vector) (+ (Transformation|GetWorldLocation (Variables|Default|GetDefaultSceneRoot)) "0, 0,30.000000")) "Undefined" 0 0))
              (Variables|/Game/Old/BP/Item_BP.Item_BP_C|Setname _returnvalue_5 (.name (Utilities|Struct|BreakResult _result)))
              (Variables|/Game/Old/BP/Item_BP.Item_BP_C|Settype _returnvalue_5 (.type (Utilities|Struct|BreakResult _result)))
              (Components|StaticMesh|SetStaticMesh (Variables|/Script/Engine.StaticMeshActor|GetStaticMeshComponent _returnvalue_5) (.MyMesh (Utilities|Struct|BreakResult _result)))
              (bind _output_get_3 (Variables|/Game/Old/BP/Item_BP.Item_BP_C|SetmaterialMain _returnvalue_5 (.materialMain (Utilities|Struct|BreakResult _result))))
              (Rendering|Material|SetMaterial (Variables|/Script/Engine.StaticMeshActor|GetStaticMeshComponent _returnvalue_5) 0 _output_get_3)
              (Effects|Components|ParticleSystem|SetTemplate (Variables|/Game/Old/BP/Item_BP.Item_BP_C|GetmyParticleSystem _returnvalue_5) (.Particle (Utilities|Struct|BreakResult _result)))
              (Rendering|SetVisibility (Variables|/Game/Old/BP/Item_BP.Item_BP_C|GetmyParticleSystem _returnvalue_5) true false)
              ;[1 1 1] Убираем воду, очищаем название
              (Rendering|SetVisibility (Variables|Default|Getcotl_water) false true)
              (Variables|Default|SetisWater? false)
              (Variables|Default|SetCurrentPotion "")
              (Actor|DestroyActor _asitem_bp)
              (Development|PrintString "5: Получилась сферка")
              (else
                ;[1 1 1] Если ничего от смешивания не вышло, то убираем воду => катализатор можно уничтожить, либо оставить в котле. Название текущего зелья стираем
                (Variables|Default|SetCurrentPotion "")
                (Variables|Default|SetisWater? false)
                (Rendering|SetVisibility (Variables|Default|Getcotl_water) false true)
                (Development|PrintString "3:От смешивания катализатора с этим ничего не вышло, катализатор ждет тебя на дне")))))
        (else
          (Development|PrintString "2: Это катализатор, но тут нет воды, пусть полежит на дне")))
      (else
        (Development|PrintString "1: Я не знаю, что это, пусть полежит на дне")))))

(fn ConstructionScript)